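; Player controller for the multiplayer Starfish Tickle Arena, handling the lobby player list, ready state, game start and forward-axis pawn movement.
; Ready changes are set locally and on the server, while join, replicated player count and state updates refresh the list.
; Start requests pass through a server event to BP_GameMode.
; Client start swaps the list for the HUD and game-only input, and game end returns to UI input.
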(event Custom|StartGameServer
  (Development|PrintString "Start server")
  (bind _asbp_game_mode (Utilities|Casting|CastToBP_GameMode (Game|GetGameMode)))
  (Default|StartGame _asbp_game_mode))

(event Custom|PlayerJoined
  (bind _playerlist (Variables|Default|GetPlayerList))
  (CallFunction|InitPlayerList)
  (Utilities|IsValid _playerlist
    (:Is%20Valid
      (Default|Refresh _playerlist))))

(event Custom|Test
  (Networking|SwitchHasAuthority
    (:Authority
      (CallFunction|PlayerJoined))))

(event Custom|StartGame
  (Development|PrintString "Start ")
  (CallFunction|StartGameServer))

(event Custom|PostLogin
  (CallFunction|InitPlayerState))

(event Custom|PlayerReadyChanged
  (params (Ready :type Boolean))
  (bind _playersstate (Variables|Default|GetPlayersState))
  (bind _playerlist (Variables|Default|GetPlayerList))
  (Utilities|FlowControl|Sequence
    (:then_0
      (Utilities|IsValid _playersstate
        (:Is%20Valid
          (Variables|/Game/StarfishTickleArena/Core/BP_PlayersState.BP_PlayersState_C|SetReady _playersstate Ready))
        (:Is%20Not%20Valid
          _))
      (CallFunction|PlayerReadyServer Ready))
    (:then_1
      (Utilities|IsValid _playerlist
        (:Is%20Valid
          (Default|Refresh _playerlist))))))

(event Custom|PlayerReadyServer
  (params (Ready :type Boolean))
  (bind _playersstate (Variables|Default|GetPlayersState))
  (Utilities|IsValid _playersstate
    (:Is%20Valid
      (Variables|/Game/StarfishTickleArena/Core/BP_PlayersState.BP_PlayersState_C|SetReady _playersstate Ready)
      (Default|CallStateUpdated _playersstate))))

(event Custom|GameEnded
  (CallFunction|InitPlayerList)
  (Input|SetInputModeUIOnly 0 (Variables|Default|GetPlayerList) "DoNotLock" false))

(event Custom|StartGameClient
  (Development|PrintString "Start client")
  (Widget|RemovefromParent (Variables|Default|GetPlayerList))
  (Input|SetInputModeGameOnly self false)
  (Variables|Default|SetbShowMouseCursor false)
  (if (Pawn|IsLocalController)
    (bind _returnvalue (UserInterface|CreateWidget "/Game/StarfishTickleArena/UI/WBP_HUD.WBP_HUD_C" 0 ""))
    (UserInterface|Viewport|AddtoViewport _returnvalue 0)))

(event Input|EnhancedActionEvents|EnhancedInputActionI_Movement
  (params (ActionValue :type Float%20%28double-precision%29) (ElapsedSeconds :type Float%20%28double-precision%29) (TriggeredSeconds :type Float%20%28double-precision%29) (InputAction :type Input%20Action%20Object%20Reference :default "/Game/StarfishTickleArena/Input/I_Movement.I_Movement"))
  (bind _returnvalue (Pawn|GetControlledPawn))
  (Pawn|Input|AddMovementInput _returnvalue (Transformation|GetActorForwardVector _returnvalue) ActionValue false))

(event EventTick
  (params (DeltaSeconds :type Float%20%28single-precision%29)))

(event EventBeginPlay
  (CallFunction|InitPlayerState)
  (if (Pawn|IsLocalPlayerController)
    (Input|AddMappingContext (PlayerController|LocalPlayerSubsystems|GetEnhancedInputLocalPlayerSubsystem) "/Game/StarfishTickleArena/Input/IMC_Bindings.IMC_Bindings" 0 "(bIgnoreAllPressedKeysUntilRelease=True,bForceImmediately=False,bNotifyUserSettings=False)")))

(fn ConstructionScript)

(fn InitPlayerList
  (if (Pawn|IsLocalPlayerController)
    (if (not (Utilities|IsValid (Variables|Default|GetPlayerList)))
      (bind _returnvalue (UserInterface|CreateWidget "/Game/StarfishTickleArena/UI/WBP_PlayerList.WBP_PlayerList_C" 0 self))
      (Variables|Default|SetPlayerList _returnvalue)
      (UserInterface|Viewport|AddtoViewport _returnvalue 0)
      (Variables|Default|SetbShowMouseCursor true))))

(fn SetPlayerName
  (params (PlayerName :type Text))
  (CallFunction|InitPlayerState)
  (Variables|/Game/StarfishTickleArena/Core/BP_PlayersState.BP_PlayersState_C|SetName (Variables|Default|GetPlayersState) ""))

(fn InitPlayerState
  (bind _playerstate (Variables|GetPlayerState))
  (Utilities|IsValid (Variables|Default|GetPlayersState)
    (:Is%20Not%20Valid
      (Utilities|IsValid _playerstate
        (:Is%20Valid
          (bind _asbp_players_state (Utilities|Casting|CastToBP_PlayersState _playerstate))
          (Variables|Default|SetPlayersState _asbp_players_state))))))

(fn OnRepPlayerCount
  (CallFunction|PlayerJoined))

(fn StateUpdated
  (bind _playerlist (Variables|Default|GetPlayerList))
  (Utilities|IsValid _playerlist
    (:Is%20Valid
      (Default|RefreshDelay _playerlist))))
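; Networked player character for Starfish Tickle Arena that crawls by placing legs and damages other players by tickling.
; Debug keys select or toggle attachment of a leg, which mouse delta moves within a clamped range; the server eases the body toward the attached legs' average.
; A server-side TickleSphere follows the moved leg, applying overlap damage until death notifies BP_GameMode.
; HP RepNotify updates the mouth material, scene-captured into a HUD render target.
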(event OnComponentBeginOverlap(TickleSphere)
  (params (OverlappedComponent :type Primitive%20Component%20Object%20Reference) (OtherActor :type Actor%20Object%20Reference) (OtherComp :type Primitive%20Component%20Object%20Reference) (OtherBodyIndex :type Integer) (bFromSweep :type Boolean) (SweepResult :type Hit%20Result%20Structure%20%28by%20ref%29))
  ;[1 1 1] if this is a player, then apply damage
  (if (not (Variables|Default|GetDead))
    (Utilities|Casting|CastToBP_PlayerController (Components|GetOwner OtherActor))
    (Game|Damage|ApplyDamage OtherActor 0.1 (Pawn|GetController) self)))

(event Custom|Init
  ;[1 1 1] INIT
  (if (not (Variables|Default|GetInited))
    (bind _asbp_player_controller (Utilities|Casting|CastToBP_PlayerController (Pawn|GetController)))
    (Variables|Default|SetPlayerController _asbp_player_controller)
    (Networking|SwitchHasAuthority
      (:Authority
        _)
      (:Remote
        (Variables|/Script/Engine.PrimitiveComponent|SetbGenerateOverlapEvents (Variables|Default|GetTickleSphere) false)))
    (if (Pawn|IsLocallyControlled)
      (bind _returnvalue (Rendering|Material|CreateDynamicMaterialInstance (Variables|Default|GetMouth) 0 0 "None" :!class /Script/Engine.PrimitiveComponent))
      (Variables|Default|SetMouthMaterial _returnvalue)
      (bind _returnvalue_2 (CanvasRenderTarget2D|CreateCanvasRenderTarget2D "/Script/Engine.CanvasRenderTarget2D" 256 256))
      (bind _output_get (Variables|Default|SetHudRender _returnvalue_2))
      (Variables|/Script/Engine.SceneCaptureComponent2D|SetTextureTarget (Variables|Default|GetSceneCaptureComponent2D) _output_get)
      (CallFunction|UpdateHP)
      (Variables|Default|SetInited true))))

(event Custom|SetPlayerLegLocation
  (if (not (Variables|Default|GetDead))
    (CallFunction|SetLegLocation (Variables|Default|GetCurrentLeg))))

(event Custom|SetActiveLeg
  (params (LegToActivate :type Integer))
  (if (not (Variables|Default|GetDead))
    (CallFunction|ActivateLeg LegToActivate)))

(event Custom|SetPlayerMousePosition
  (params (PlayerMouseVector :type Vector))
  (Variables|Default|SetPlayerMouseVector PlayerMouseVector))

(event Custom|FlipPlayerAttachStatus
  (CallFunction|FlipAttachStatus))

(event EventBeginPlay
  ;[1 1 1] INIT
  (if (not (Variables|Default|GetInited))
    (bind _asbp_player_controller (Utilities|Casting|CastToBP_PlayerController (Pawn|GetController)))
    (Variables|Default|SetPlayerController _asbp_player_controller)
    (Networking|SwitchHasAuthority
      (:Authority
        _)
      (:Remote
        (Variables|/Script/Engine.PrimitiveComponent|SetbGenerateOverlapEvents (Variables|Default|GetTickleSphere) false)))
    (if (Pawn|IsLocallyControlled)
      (bind _returnvalue (Rendering|Material|CreateDynamicMaterialInstance (Variables|Default|GetMouth) 0 0 "None" :!class /Script/Engine.PrimitiveComponent))
      (Variables|Default|SetMouthMaterial _returnvalue)
      (bind _returnvalue_2 (CanvasRenderTarget2D|CreateCanvasRenderTarget2D "/Script/Engine.CanvasRenderTarget2D" 256 256))
      (bind _output_get (Variables|Default|SetHudRender _returnvalue_2))
      (Variables|/Script/Engine.SceneCaptureComponent2D|SetTextureTarget (Variables|Default|GetSceneCaptureComponent2D) _output_get)
      (CallFunction|UpdateHP)
      (Variables|Default|SetInited true))))

(event Collision|EventActorBeginOverlap
  (params (OtherActor :type Actor%20Object%20Reference)))

(event EventTick
  (params (DeltaSeconds :type Float%20%28single-precision%29))
  (if (not (Variables|Default|GetDead))
    (Utilities|FlowControl|Sequence
      (:then_0
        (if (Pawn|IsLocallyControlled)
          (if (Variables|Default|GetIsLegActive)
            (bind _mousevector (CallFunction|GetMousePosition))
            (CallFunction|SetPlayerMousePosition _mousevector)
            (CallFunction|SetPlayerLegLocation)
            (CallFunction|DrawDebugSpheresonLegs))))
      (:then_1
        (Networking|SwitchHasAuthority
          (:Authority
            (CallFunction|MovePlayer DeltaSeconds)))))))

(event Game|Damage|EventAnyDamage
  (params (Damage :type Float%20%28single-precision%29) (DamageType :type Damage%20Type%20Object%20Reference) (InstigatedBy :type Controller%20Object%20Reference) (DamageCauser :type Actor%20Object%20Reference))
  (if (not (Variables|Default|GetDead))
    (CallFunction|ApplyDamageTaken Damage)))

(event Input|KeyboardEvents|DebugKey1
  (params (Key :type Key%20Structure :default "None") (ActionValue :type Input%20Action%20Value%20Structure))
  ;[1 1 1] Inputs
  (:Pressed
    (CallFunction|SetActiveLeg)))

(event Input|KeyboardEvents|DebugKey2
  (params (Key :type Key%20Structure :default "None") (ActionValue :type Input%20Action%20Value%20Structure))
  ;[1 1 1] Inputs
  (:Pressed
    (CallFunction|SetActiveLeg 1)))

(event Input|KeyboardEvents|DebugKey3
  (params (Key :type Key%20Structure :default "None") (ActionValue :type Input%20Action%20Value%20Structure))
  ;[1 1 1] Inputs
  (:Pressed
    (CallFunction|SetActiveLeg 2)))

(event Input|KeyboardEvents|DebugKey7
  (params (Key :type Key%20Structure :default "None") (ActionValue :type Input%20Action%20Value%20Structure)))

(event Input|KeyboardEvents|DebugKey5
  (params (Key :type Key%20Structure :default "None") (ActionValue :type Input%20Action%20Value%20Structure))
  ;[1 1 1] Inputs
  (:Pressed
    (CallFunction|FlipPlayerAttachStatus)))

(fn ConstructionScript
  (CallFunction|InitSetLegLocations)
  (Variables|Default|SetBoneInit true))

(fn InitSetLegLocations
  (bind _legs (Variables|Default|GetLegs))
  (for (_array_element _array_index) _legs
    (Utilities|Array|SetArrayElem _legs _array_index (Math|Transform|TransformLocation (Transformation|GetActorTransform) _array_element))))

(fn GetMouseinWorldPosition
  (bind _playercontroller (Variables|Default|GetPlayerController))
  (bind (_worldlocation _worlddirection) (Game|Player|ConvertMouseLocationToWorldSpace _playercontroller))
  (bind _outhit (Collision|LineTraceByChannel (Transformation|GetActorLocation (Variables|/Script/Engine.PlayerController|GetPlayerCameraManager _playercontroller)) (+ _worldlocation (* _worlddirection 1e+04)) "TraceTypeQuery1" false 0 "None"))
  (if (.bBlockingHit (Collision|BreakHitResult _outhit))
    (return (.Location (Collision|BreakHitResult _outhit)))
    (else
      (Development|PrintString "ERROR: Mouse position not found" true true "(R=1.000000,G=0.000000,B=0.014359,A=1.000000)" 1e+01))))

(fn GetMousePosition
  (bind _playercontroller (Variables|Default|GetPlayerController))
  (bind (_deltax _deltay) (Class|PlayerController|GetInputMouseDelta _playercontroller))
  (return (Math|Vector|MakeVector 0.0 _deltax _deltay)))

(fn SetLegLocation
  (params (LegNumber :type Integer))
  (bind _legs (Variables|Default|GetLegs))
  (bind _maxrange (Variables|Default|GetMaxRange))
  (bind _mesh (Variables|Character|GetMesh))
  (bind _playermousevector (Variables|Default|GetPlayerMouseVector))
  (bind _returnvalue (Transformation|GetWorldLocation _mesh))
  (bind _output (Utilities|Array|Get(acopy) _legs LegNumber))
  (bind _returnvalue_2 (+ _output _playermousevector))
  (bind _returnvalue_3 (- _returnvalue_2 _returnvalue))
  (bind _returnvalue_4 (Math|Vector|ClampVectorSize _returnvalue_3 0.0 _maxrange))
  (bind _returnvalue_5 (+ _returnvalue_4 _returnvalue))
  (Utilities|Array|SetArrayElem _legs LegNumber _returnvalue_5)
  (Networking|SwitchHasAuthority
    (:Authority
      (Transformation|SetWorldLocation (Variables|Default|GetTickleSphere) _returnvalue_5 false false))))

(fn ActivateLeg
  (params (LegToActivate :type Integer))
  (for (_array_element _array_index) (Variables|Default|GetLegsAttached)
    (if _array_element
      (if (!= _array_index LegToActivate)
        (bind _result (Math|Integer|IncrementInt (LocalVariables|GetActiveLegs))
          (:%20%20
            (LocalVariables|SetActiveLegs _result))))))
  (if (> (LocalVariables|GetActiveLegs) 0)
    (Variables|Default|SetCurrentLeg LegToActivate)
    (Variables|Default|SetInitialLegPosition (Utilities|Array|Get(acopy) (Variables|Default|GetLegs) (Variables|Default|GetCurrentLeg)))
    (Variables|Default|SetIsLegActive true)
    (Utilities|Array|SetArrayElem (Variables|Default|GetLegsAttached) (Variables|Default|GetCurrentLeg) false)))

(fn FlipAttachStatus
  (bind _currentleg (Variables|Default|GetCurrentLeg))
  (bind _legsattached (Variables|Default|GetLegsAttached))
  (bind _legs (Variables|Default|GetLegs))
  (bind _currentleg_2 (Variables|Default|GetCurrentLeg))
  (bind _output (Utilities|Array|Get(acopy) _legs _currentleg_2))
  (bind (_outhits _returnvalue) (Collision|MultiSphereTraceByChannel _output _output (LocalVariables|GetColisionRadiusCheck) "TraceTypeQuery1" false 0 "None"))
  (if _returnvalue
    (for _array_element _outhits
      (Utilities|Array|SetArrayElem _legsattached _currentleg (not (Utilities|Array|Get(acopy) _legsattached _currentleg)))
      (Variables|Default|SetIsLegActive false))))

(fn GetAttachedLegsLocation
  (bind _legsattached (Variables|Default|GetLegsAttached))
  (bind _legslocation (LocalVariables|GetLegsLocation))
  (for (_ _array_index) _legsattached
    (if (Utilities|Array|Get(acopy) _legsattached _array_index)
      (Utilities|Array|Add (LocalVariables|GetLegsLocation) (Utilities|Array|Get(acopy) (Variables|Default|GetLegs) _array_index))))
  (if (not (== (Utilities|Array|Length _legslocation) 0))
    (return (Math|Vector|GetVectorArrayAverage _legslocation))))

(fn DrawDebugSpheresonLegs
  (for (_array_element _array_index) (Variables|Default|GetLegs)
    (if (Utilities|Array|Get(acopy) (Variables|Default|GetLegsAttached) _array_index)
      (Rendering|Debug|DrawDebugSphere _array_element 1e+01 8 "(R=0.014992,G=1.000000,B=0.000000,A=1.000000)" 0.0 2.0)
      (else
        (Rendering|Debug|DrawDebugSphere _array_element 1e+01 8 "(R=1.000000,G=0.000000,B=0.000000,A=1.000000)" 0.0 2.0)))))

(fn MovePlayer
  (params (DeltaTime :type Float%20%28double-precision%29))
  (bind _centeredlocation (CallFunction|GetAttachedLegsLocation))
  (Transformation|SetActorLocation (Math|Interpolation|VInterpTo (Transformation|GetActorLocation) _centeredlocation DeltaTime 1.0) false false))

(fn UpdateHP
  (bind _mouthmaterial (Variables|Default|GetMouthMaterial))
  (Utilities|IsValid _mouthmaterial
    (:Is%20Valid
      (Rendering|Material|SetScalarParameterValue _mouthmaterial "HPPercent" (Math|Float|Clamp(Float) (Variables|Default|GetHP)) :!class /Script/Engine.MaterialInstanceDynamic)
      (Rendering|SceneCapture|CaptureScene (Variables|Default|GetSceneCaptureComponent2D) :!class /Script/Engine.SceneCaptureComponent2D))))

(fn ApplyDamageTaken
  (params (DamageTaken :type Float%20%28double-precision%29))
  ;[1 1 1] dont do shit if hp is less than 0
  (if (not (<= (Variables|Default|GetHP) 0.0))
    ;[1 1 1] is this the killing blow?
    (if (<= (- (Variables|Default|GetHP) DamageTaken) 0.0)
      (Variables|Default|SetDead true)
      (Variables|Default|SetHP 0.0)
      (bind _asbp_game_mode (Utilities|Casting|CastToBP_GameMode (Game|GetGameMode)))
      (Default|PlayerDied _asbp_game_mode)
      (else
        (Variables|Default|SetHP (- (Variables|Default|GetHP) DamageTaken))))))

(fn OnRepHP
  (CallFunction|UpdateHP))